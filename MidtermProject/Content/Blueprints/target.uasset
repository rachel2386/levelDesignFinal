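; Target actor whose cube jumps through a fixed sequence of six relative positions as myCharacter overlaps it, starting at the first on BeginPlay.
; On overlap, it compares the cube's location against the stored positions to set PositionIndex.
; Tick reapplies the following position for that index through SetNewTargetPos, without interpolation or sweep.
; The sequence ends at the sixth position, with no wraparound.
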(event EventBeginPlay
  (CallFunction|SetNewTargetPos (Variables|Default|Getpos1)))

(event Collision|EventActorBeginOverlap
  (params (OtherActor :type Actor%20Object%20Reference))
  (Utilities|Casting|CastTomyCharacter OtherActor)
  (if (Math|Vector|Equal(Vector) (Variables|/Script/Engine.SceneComponent|GetRelativeLocation (Variables|Default|GetCube)) (Variables|Default|Getpos1) 1.0)
    (Variables|Default|SetpositionIndex 1)
    (elif (Math|Vector|Equal(Vector) (Variables|/Script/Engine.SceneComponent|GetRelativeLocation (Variables|Default|GetCube)) (Variables|Default|Getpos2) 0.1)
      (Variables|Default|SetpositionIndex 2)
      (elif (Math|Vector|Equal(Vector) (Variables|/Script/Engine.SceneComponent|GetRelativeLocation (Variables|Default|GetCube)) (Variables|Default|Getpos3) 0.1)
        (Variables|Default|SetpositionIndex 3)
        (elif (Math|Vector|Equal(Vector) (Variables|/Script/Engine.SceneComponent|GetRelativeLocation (Variables|Default|GetCube)) (Variables|Default|Getpos4) 0.1)
          (Variables|Default|SetpositionIndex 4)
          (elif (Math|Vector|Equal(Vector) (Variables|/Script/Engine.SceneComponent|GetRelativeLocation (Variables|Default|GetCube)) (Variables|Default|Getpos5) 0.1)
            (Variables|Default|SetpositionIndex 5)
            (elif (Math|Vector|Equal(Vector) (Variables|/Script/Engine.SceneComponent|GetRelativeLocation (Variables|Default|GetCube)) (Variables|Default|Getpos6) 0.1)
              (Variables|Default|SetpositionIndex 6))))))))

(event EventTick
  (params (DeltaSeconds :type Float%20%28single-precision%29))
  (switch int (Variables|Default|GetpositionIndex)
    (:1
      (CallFunction|SetNewTargetPos (Variables|Default|Getpos2)))
    (:2
      (CallFunction|SetNewTargetPos (Variables|Default|Getpos3)))
    (:3
      (CallFunction|SetNewTargetPos (Variables|Default|Getpos4)))
    (:4
      (CallFunction|SetNewTargetPos (Variables|Default|Getpos5)))
    (:5
      (CallFunction|SetNewTargetPos (Variables|Default|Getpos6)))))

(fn ConstructionScript)

(fn SetNewTargetPos
  (params (newPos :type Vector))
  (Transformation|SetRelativeLocation (Variables|Default|GetCube) newPos false false))